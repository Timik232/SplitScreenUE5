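; BP_Projectile is a projectile actor in the SplitScreen game folder that damages what it overlaps and pushes physics objects.
; On sphere overlap with anything other than itself or its Instigator, it sends a GetDamageMessage carrying damage and its velocity, then destroys itself.
; Hitting a physics-simulating component applies a forward impulse and destroys it, as does the projectile movement stopping.
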(event OnComponentBeginOverlap(SphereCollision)
  (params (OverlappedComponent :type Primitive%20Component%20Object%20Reference) (OtherActor :type Actor%20Object%20Reference) (OtherComp :type Primitive%20Component%20Object%20Reference) (OtherBodyIndex :type Integer) (bFromSweep :type Boolean) (SweepResult :type Hit%20Result%20Structure%20%28by%20ref%29))
  (if (not (or (== OtherActor self) (== OtherActor (Game|GetInstigator))))
    (Class|BPIDamagable|GetDamage(Message) OtherActor 1 (Variables|/Script/Engine.MovementComponent|GetVelocity (Variables|Default|GetProjectileMovement)))
    (Actor|DestroyActor)))

(event OnProjectileStop(ProjectileMovement)
  (params (ImpactResult :type Hit%20Result%20Structure%20%28by%20ref%29))
  (Actor|DestroyActor))

(event OnComponentHit(SphereCollision)
  (params (HitComponent :type Primitive%20Component%20Object%20Reference) (OtherActor :type Actor%20Object%20Reference) (OtherComp :type Primitive%20Component%20Object%20Reference) (NormalImpulse :type Vector :default "0, 0, 0") (Hit :type Hit%20Result%20Structure%20%28by%20ref%29))
  (if (Physics|IsSimulatingPhysics OtherComp "None")
    (Physics|AddImpulse OtherComp (* (Math|Vector|GetForwardVector (Variables|Default|GetSphereCollision)) 1.3e+04) "None" false)
    (Actor|DestroyActor)))

(event EventBeginPlay)

(event Collision|EventActorBeginOverlap
  (params (OtherActor :type Actor%20Object%20Reference)))

(event EventTick
  (params (DeltaSeconds :type Float%20%28single-precision%29)))

(fn ConstructionScript)