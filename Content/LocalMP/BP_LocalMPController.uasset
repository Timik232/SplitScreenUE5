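; Player controller for local splitscreen tank multiplayer that handles input, per-player HUD, tank color and the game-over screen.
; Adds the splitscreen mapping context and forwards move, rotate and shoot input to the pawn as messages.
; Looks up color in DT_PlayerInfo by player name, applies it on possess, and displays zero-based player names plus one.
; SetIndex separately builds a HUD and tints BP_TopDownCharacter; click-to-move helpers are not called here.
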(event Custom|UpdateNameUI
  (bind _widgethud (Variables|Default|GetWidgetHUD)
    (:then
      (Rendering|Components|TextRender|SetText (Variables|/Game/SplitScreen/WBP_HUD.WBP_HUD_C|GetPlayerNumber _widgethud) (Utilities|Text|ToText(String) (Variables|Default|GetPlayerName))))
    (:else)))

(event Custom|HandlePlayerWin
  (params (WinnerState :type Player%20State%20Object%20Reference))
  (bind _returnvalue (UserInterface|CreateWidget "/Game/LocalMP/WBP_GameOverLocalMP.WBP_GameOverLocalMP_C" 0 (Utilities|Text|ToText(String) (Utilities|String|ToString(Integer) (+ (Math|Conversions|ToInteger(Byte) (PlayerState|GetPlayerName WinnerState)) 1)))))
  (UserInterface|Viewport|AddtoViewport _returnvalue 0)
  (Input|SetInputModeUIOnly self _returnvalue "DoNotLock" false)
  (Variables|Default|SetbShowMouseCursor true))

(event Custom|UpdateColor
  (bind _returnvalue (Utilities|GetDataTableRow "/Game/SplitScreen/DT_PlayerInfo.DT_PlayerInfo" (Utilities|String|StringToName (PlayerState|GetPlayerName (Variables|GetPlayerState))))
    (:then
      (Variables|Default|SetTankColor _returnvalue))))

(event Custom|TryUpdateMeshColor
  (params (Object :type Object%20Object%20Reference))
  (bind _asbp_local_mpcharacter (Utilities|Casting|CastToBP_LocalMPCharacter Object))
  (Default|SetTankColor _asbp_local_mpcharacter (Variables|Default|GetTankColor)))

(event Custom|Update%20Health%20UI
  (params (HP :type Float%20%28double-precision%29))
  (Rendering|Components|TextRender|SetText (Variables|/Game/SplitScreen/WBP_HUD.WBP_HUD_C|GetPlayerHP (Variables|Default|GetWidgetHUD)) (Utilities|Text|ToText(Integer) (Math|Float|Round HP))))

(event Custom|UpdateName
  (params (NewName :type String))
  (Variables|Default|SetPlayerName (Utilities|String|ToString(Integer) (+ (Math|Conversions|ToInteger(Byte) NewName) 1)))
  (CallFunction|UpdateNameUI))

(event Input|EnhancedActionEvents|EnhancedInputActionIA_Shoot1
  (params (ActionValue :type Boolean) (ElapsedSeconds :type Float%20%28double-precision%29) (TriggeredSeconds :type Float%20%28double-precision%29) (InputAction :type Input%20Action%20Object%20Reference :default "/Game/SplitScreen/Actions/IA_Shoot1.IA_Shoot1"))
  (:Started
    (Class|BPIControllable|ProcessShoot(Message) (Pawn|GetControlledPawn))))

(event Input|EnhancedActionEvents|EnhancedInputActionIA_MoveForward1
  (params (ActionValue :type Boolean) (ElapsedSeconds :type Float%20%28double-precision%29) (TriggeredSeconds :type Float%20%28double-precision%29) (InputAction :type Input%20Action%20Object%20Reference :default "/Game/SplitScreen/Actions/IA_MoveForward1.IA_MoveForward1"))
  (Class|BPIControllable|ProcessMoveForward(Message) (Pawn|GetControlledPawn)))

(event Input|EnhancedActionEvents|EnhancedInputActionIA_Rotation1
  (params (ActionValue :type Float%20%28double-precision%29) (ElapsedSeconds :type Float%20%28double-precision%29) (TriggeredSeconds :type Float%20%28double-precision%29) (InputAction :type Input%20Action%20Object%20Reference :default "/Game/SplitScreen/Actions/IA_Rotation1.IA_Rotation1"))
  (Class|BPIControllable|ProcessRotation(Message) (Pawn|GetControlledPawn) ActionValue))

(event EventBeginPlay
  (bind _returnvalue (PlayerController|LocalPlayerSubsystems|GetEnhancedInputLocalPlayerSubsystem))
  ;[0.05098 0.05098 0.05098] Add Mapping Context
  (Utilities|IsValid _returnvalue
    (:Is%20Valid
      (Input|AddMappingContext _returnvalue "/Game/SplitScreen/Actions/IMC_Splitscreen.IMC_Splitscreen" 0 "(bIgnoreAllPressedKeysUntilRelease=True,bForceImmediately=False,bNotifyUserSettings=False)")
      (Input|SetInputModeGameOnly self false)
      (Variables|Default|SetbShowMouseCursor false)
      (bind _returnvalue_2 (UserInterface|CreateWidget "/Game/SplitScreen/WBP_HUD.WBP_HUD_C" self))
      (bind _output_get (Variables|Default|SetWidgetHUD _returnvalue_2))
      (UserInterface|Viewport|AddtoViewport _output_get 0)
      (CallFunction|UpdateNameUI))))

(event EventPossess
  (params (PossessedPawn :type Pawn%20Object%20Reference))
  (CallFunction|TryUpdateMeshColor PossessedPawn))

(fn ConstructionScript)

(fn Moveto
  (params (Location :type Vector))
  (AI|Navigation|SimpleMovetoLocation self Location)
  (Niagara|SpawnSystematLocation (Variables|Input|GetFXCursor) Location))

(fn Follow
  (params (Location :type Vector))
  (bind _returnvalue (Pawn|GetControlledPawn))
  (Pawn|Input|AddMovementInput _returnvalue (Math|Vector|GetUnitDirection(Vector) (Transformation|GetActorLocation _returnvalue) Location) 1.0 false))

(fn GetLocationUnderCursor
  (bind _hitresult (Game|Player|GetHitResultUnderCursorbyChannel "TraceTypeQuery1" true))
  (bind (_bblockinghit _binitialoverlap _time _distance _location) (Collision|BreakHitResult _hitresult))
  (return _bblockinghit _location))

(fn GetLocationUnderFinger
  (bind _hitresult (Class|PlayerController|GetHitResultUnderFingerbyChannel "Touch1" "TraceTypeQuery1" false))
  (bind (_bblockinghit _binitialoverlap _time _distance _location) (Collision|BreakHitResult _hitresult))
  (return _bblockinghit _location))

(fn SetIndex
  (params (Index :type Integer))
  (bind _returnvalue (UserInterface|CreateWidget "/Game/SplitScreen/WBP_HUD.WBP_HUD_C" self))
  (UserInterface|Viewport|AddtoPlayerScreen _returnvalue)
  (bind _output_get (Variables|Default|SetWidgetHUD _returnvalue))
  (Rendering|Components|TextRender|SetText (Variables|/Game/SplitScreen/WBP_HUD.WBP_HUD_C|GetPlayerNumber _output_get) (Utilities|Text|ToText(Integer) (+ 1 Index)))
  (bind _asbp_top_down_character (Utilities|Casting|CastToBP_TopDownCharacter (Pawn|GetControlledPawn)))
  (bind _returnvalue_2 (Rendering|Material|CreateDynamicMaterialInstance (Variables|/Game/SplitScreen/BP_TopDownCharacter.BP_TopDownCharacter_C|Getpoteha_tank _asbp_top_down_character) 0 "/Game/SplitScreen/M_MasterMaterial.M_MasterMaterial" "None" :!class /Script/Engine.PrimitiveComponent))
  (bind _returnvalue_3 (Utilities|GetDataTableRow "/Game/SplitScreen/DT_PlayerInfo.DT_PlayerInfo" (Utilities|String|StringToName (Utilities|String|ToString(Integer) Index)))
    (:then
      (Rendering|Material|SetVectorParameterValue _returnvalue_2 "Color" (Utilities|Struct|BreakS_PlayerInfo _returnvalue_3) :!class /Script/Engine.MaterialInstanceDynamic))))