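; Game mode for local multiplayer that tracks living players to decide a last-player-standing winner.
; On login, each player joins the AlivePlayers array and, for local multiplayer controllers, is renamed to the returned array index.
; Logout routes into MarkPlayerAsDead, which removes an entry and, when one or none remain, passes the first entry's PlayerState to the cached game state's ProcessPlayerWin.
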(event Custom|MarkPlayerAsDead
  (params (DeadPlayer :type Controller%20Object%20Reference%20%28by%20ref%29))
  (bind _aliveplayers (Variables|Default|GetAlivePlayers))
  (bind _output (Utilities|Array|Get(acopy) _aliveplayers))
  (Utilities|Array|RemoveItem (Variables|Default|GetAlivePlayers) 0)
  (if (<= (Utilities|Array|Length _aliveplayers) 1)
    (Utilities|Casting|CastToBP_LocalMPController _output)
    (Default|ProcessPlayerWin (Variables|Default|GetMPGameState) (Variables|/Script/Engine.Controller|GetPlayerState _output))))

(event EventBeginPlay
  (Utilities|Casting|CastToBP_TopDownGameInstance (Game|GetGameInstance))
  (bind _asbp_local_mpgame_state (Utilities|Casting|CastToBP_LocalMPGameState (Game|GetGameState)))
  (Variables|Default|SetMPGameState _asbp_local_mpgame_state))

(event EventPostLogin
  (params (NewPlayer :type Player%20Controller%20Object%20Reference))
  (bind _returnvalue (Utilities|Array|Add (Variables|Default|GetAlivePlayers) NewPlayer))
  (bind _asbp_local_mpcontroller (Utilities|Casting|CastToBP_LocalMPController NewPlayer))
  (Class|GameModeBase|ChangeName _asbp_local_mpcontroller (Utilities|String|ToString(Integer) _returnvalue) true))

(event EventOnLogout
  (params (ExitingController :type Controller%20Object%20Reference))
  (CallFunction|MarkPlayerasDead ExitingController))

(fn ConstructionScript)