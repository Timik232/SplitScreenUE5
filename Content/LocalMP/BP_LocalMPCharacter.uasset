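; Player character for local multiplayer that drives forward, turns, shoots projectiles and toggles between near and far spring-arm camera distances.
; It registers its controller with the game mode, and a delay-based reload flag limits firing from GunShooter.
; Damage compares hit direction to facing, ignoring hits within 45 degrees of head-on.
; Other hits reduce HP, update the controller's health UI, and at zero destroy the actor and notify the game state.
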(event Custom|ChangeCameraDistance
  (params (bUseFarCamera :type Boolean))
  (Variables|/Script/Engine.SpringArmComponent|SetTargetArmLength (Variables|Camera|GetSpringArm) (select bUseFarCamera 2.5e+03 1.4e+03)))

(event Custom|TryShoot
  (bind _self self)
  (bind _gunshooter (Variables|Default|GetGunShooter))
  (if (not (Variables|Default|GetbOnReload))
    (Game|SpawnActorfromClass "/Game/SplitScreen/BP_Projectile.BP_Projectile_C" (Math|Transform|MakeTransform (Transformation|GetWorldLocation _gunshooter) (Transformation|GetWorldRotation _gunshooter)) "Undefined" "MultiplyWithRoot" _self _self)
    (Variables|Default|SetbOnReload true)
    (Utilities|FlowControl|Delay (Variables|Default|GetReloadTime))
    (Variables|Default|SetbOnReload false)))

(event Custom|ProcessDamage
  (params (HitDirection :type Vector))
  (bind _returnvalue (Math|Conversions|RotationFromXVector HitDirection))
  (bind _capsulecomponent (Variables|Collision|GetCapsuleComponent))
  (bind _returnvalue_2 (Math|Vector|GetForwardVector _capsulecomponent))
  (bind _returnvalue_3 (Math|Vector|NegateVector _returnvalue_2))
  (bind _returnvalue_4 (Math|Conversions|RotationFromXVector _returnvalue_3))
  (bind _returnvalue_5 (Math|Rotator|Delta(Rotator) _returnvalue _returnvalue_4))
  (bind _yaw (Math|Rotator|BreakRotator _returnvalue_5))
  (bind _returnvalue_6 (Math|Float|Absolute(Float) _yaw))
  (bind _returnvalue_7 (< _returnvalue_6 45.0))
  (if (not _returnvalue_7)
    (bind _output_get (Variables|Default|SetHP (Math|Float|Max(Float) (- (Variables|Default|GetHP) (Math|Float|SelectFloat 1.0 2.0 _returnvalue_7)) 0.0)))
    (bind _asbp_local_mpcontroller (Utilities|Casting|CastToBP_LocalMPController (Pawn|GetController)))
    (Default|UpdateHealthUI _asbp_local_mpcontroller _output_get)
    (if (<= (Variables|Default|GetHP) 0.0)
      (Actor|DestroyActor)
      (bind _asbp_local_mpgame_state (Utilities|Casting|CastToBP_LocalMPGameState (Game|GetGameState)))
      (Default|KillPlayer _asbp_local_mpgame_state (Pawn|GetController)))))

(event EventProcessMoveForward
  (Class|PawnMovementComponent|AddInputVector (Variables|Character|GetCharacterMovement) (* (Math|Vector|GetForwardVector (Variables|Collision|GetCapsuleComponent)) (Variables|Default|GetSpeed) (Utilities|Time|GetWorldDeltaSeconds)) false))

(event EventProcessShoot
  (if (not (Variables|Default|GetbOnReload))
    (CallFunction|TryShoot)))

(event EventProcessRotation
  (params (Direction :type Float%20%28double-precision%29))
  (Class|Actor|AddActorWorldRotation (Math|Rotator|MakeRotator 0.0 0.0 (* Direction (Variables|Default|GetRotationSpeed) (Utilities|Time|GetWorldDeltaSeconds)))))

(event EventBeginPlay
  (Utilities|FlowControl|DelayUntilNextTick)
  (bind _asbp_top_down_game_mode (Utilities|Casting|CastToBP_TopDownGameMode (Game|GetGameMode)))
  (bind _asplayer_controller (Utilities|Casting|CastToPlayerController (Pawn|GetController)))
  (Utilities|Array|Add (Variables|/Game/SplitScreen/BP_TopDownGameMode.BP_TopDownGameMode_C|GetPlayerControllers _asbp_top_down_game_mode) _asplayer_controller))

(event EventGetDamage
  (params (Damage :type Integer) (Vector :type Vector :default "0, 0, 0"))
  (CallFunction|ProcessDamage Vector))

(fn ConstructionScript)